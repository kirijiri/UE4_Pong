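; BP_Ball_Menu is a bouncing ball actor, apparently for the menu, launched diagonally across the XY plane on BeginPlay.
; It bounces by overlap events, negating its StaticMesh physics velocity in X on BP_horizontalWall and in Y on BP_Goal_L.
; Other overlapping actors are ignored.
; Collision sound spawn nodes are present but unconnected, so they never play.
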(event `self.ReceiveBeginPlay`
  (`PrimitiveComponent.SetPhysicsLinearVelocity` (`self.StaticMesh`) (2000.0 2000.0 0.0) false "None"))

(event `self.ReceiveActorBeginOverlap`
  (params (OtherActor :type "Actor Object Reference"))
  (cast `/Game/Blueprints/BP_horizontalWall` OtherActor
    (:`then`
      (bind _returnvalue (`PrimitiveComponent.GetPhysicsLinearVelocity` (`self.StaticMesh`) "None"))
      (`PrimitiveComponent.SetPhysicsLinearVelocity` (`self.StaticMesh`) (`KismetMathLibrary.MakeVector` (* (.x _returnvalue) -1.0) (.y _returnvalue) (.z _returnvalue)) false "None"))
    (:`CastFailed`
      (cast `/Game/Blueprints/BP_Goal_L` OtherActor)
      (bind _returnvalue_2 (`PrimitiveComponent.GetPhysicsLinearVelocity` (`self.StaticMesh`) "None"))
      (`PrimitiveComponent.SetPhysicsLinearVelocity` (`self.StaticMesh`) (`KismetMathLibrary.MakeVector` (.x _returnvalue_2) (* (.y _returnvalue_2) -1.0) (.z _returnvalue_2)) false "None"))))

(fn `UserConstructionScript`)