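; Left paddle Blueprint that slides along the world X axis under player two's P2_Move input.
; Each Tick pushes PaddleMesh with a physics force scaled by that input.
; When the paddle passes either symmetric X limit, it is snapped back to the limit without sweep, and no force is applied that frame.
; Velocity is not reset on the snap.
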(event `self.ReceiveTick`
  (params (DeltaSeconds :type "Float (single-precision)"))
  (if (> (.x (`self.K2_GetActorLocation`)) 1200.0)
    (`self.K2_SetActorLocation` (`KismetMathLibrary.MakeVector` 1200.0 (.y (`self.K2_GetActorLocation`)) (.z (`self.K2_GetActorLocation`))))
    (elif (< (.x (`self.K2_GetActorLocation`)) -1200.0)
      (`self.K2_SetActorLocation` (`KismetMathLibrary.MakeVector` -1200.0 (.y (`self.K2_GetActorLocation`)) (.z (`self.K2_GetActorLocation`))))
      (else
        (`PrimitiveComponent.AddForce` (`self.Paddle_Mesh`) (`KismetMathLibrary.MakeVector` (* (`self.GetInputAxisValue`) 9000000.0)) "None" false)))))

(fn `UserConstructionScript`)